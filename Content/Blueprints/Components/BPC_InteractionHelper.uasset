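; BPC_InteractionHelper is a helper component that supports highlighting of interactable objects.
; Its begin and end overlap events forward the given Owner to overlapping actors that implement BPI_HighlightInteraction.
; A separate message event sets or clears the MI_ObjectHighlight overlay material on the Owner's static mesh component based on CanInteract, printing a debug string on each call.
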(event `MyBeginOverlap`
  (params (OverlapActor :type "Actor Object Reference") (Owner :type "Actor Object Reference"))
  (if (`KismetSystemLibrary.DoesImplementInterface` OverlapActor "/Game/Blueprints/BPI_HighlightInteraction.BPI_HighlightInteraction_C")
    (message `/Game/Blueprints/BPI_HighlightInteraction.BeginOverlap` OverlapActor Owner)))

(event `MyEndOverlap`
  (params (OverlapActor :type "Actor Object Reference") (Owner :type "Actor Object Reference"))
  (if (`KismetSystemLibrary.DoesImplementInterface` OverlapActor "/Game/Blueprints/BPI_HighlightInteraction.BPI_HighlightInteraction_C")
    (message `/Game/Blueprints/BPI_HighlightInteraction.EndOverlap` OverlapActor Owner)))

(event `MyInterfaceMessage`
  (params (bCanInteract :type Boolean) (Owner :type "Actor Object Reference"))
  (bind _returnvalue (`Actor.GetComponentByClass` Owner "/Script/Engine.StaticMeshComponent"))
  (`KismetSystemLibrary.PrintString` "OverlayON")
  (if bCanInteract
    (`MeshComponent.SetOverlayMaterial` _returnvalue "/Game/Materials/MI_ObjectHighlight.MI_ObjectHighlight")
    (else
      (`MeshComponent.SetOverlayMaterial` _returnvalue null))))