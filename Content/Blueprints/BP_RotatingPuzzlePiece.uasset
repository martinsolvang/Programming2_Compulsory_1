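; BP_RotatingPuzzlePiece is an interactable puzzle piece whose static mesh turns 90 degrees in yaw when used.
; OnInteract passes a DoOnce gate, stores the current world rotation and plays a timeline that lerps the added yaw, setting pitch and roll to zero.
; The gate is reset through a one-second Delay fired from the timeline's Update output rather than Finished, so re-interaction timing is independent of the timeline's end.
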(event `Interact_Interface.OnInteract`
  (bind (_initialrotation_roll _initialrotation_pitch _initialrotation_yaw) (`KismetMathLibrary.BreakRotator` (`self.InitialRotation`)))
  (`/Engine/EditorBlueprintResources/StandardMacros.DoOnce` false :!label _label
    (:`Completed`
      (`KismetSystemLibrary.PrintString` "Rotated")
      (set `self.InitialRotation` (`SceneComponent.K2_GetComponentRotation` (`self.StaticMesh`)))
      (bind (_direction _newtrack_0) (`Timeline|Rotate` :!via `PlayFromStart`)
        (:`Update`
          (`SceneComponent.K2_SetWorldRotation` (`self.StaticMesh`) (`KismetMathLibrary.MakeRotator` 0.0 0.0 (+ (`KismetMathLibrary.Lerp` 0.0 90.0 _newtrack_0) _initialrotation_yaw)) false false)
          (`KismetSystemLibrary.Delay` 1.0)
          (goto _label :!via `Reset`))))))

(fn `UserConstructionScript`)