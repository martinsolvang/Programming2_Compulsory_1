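; BP_RotatingPuzzlePiece is a puzzle piece meant to rotate its static mesh in 90-degree yaw steps, though no event triggers that logic.
; The unconnected chain passes a DoOnce, stores the current rotation and plays the Rotate timeline to lerp yaw from it, zeroing pitch and roll.
; A Delay on the timeline's Update resets the DoOnce to allow another turn.
; The construction script is empty.
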(fn `UserConstructionScript`)