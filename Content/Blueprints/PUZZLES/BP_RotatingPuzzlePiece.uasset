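; BP_RotatingPuzzlePiece is a puzzle piece Blueprint meant to turn its static mesh 90 degrees in yaw, but no event triggers that logic.
; The unconnected chain passes a DoOnce, prints a debug string, stores the world rotation and plays the Rotate timeline.
; Timeline updates lerp yaw from the stored value, zero pitch and roll, and lead into a Delay that resets the DoOnce.
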(fn `UserConstructionScript`)