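; Test submarine actor that shows a crosshair and reacts to geyser hazard zones.
; A FlipFlop on EnteredHazardZone toggles boosted movement speed and acceleration, while Tick applies the geyser's force vector as movement input.
; A looping-timer routine is built to highlight the interactable nearest the Arrow, but its overlap tracking is disconnected.
; Interact and projectile-shooting logic is also unwired, leaving both input events empty.
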(event `self.ReceiveBeginPlay`
  (bind _returnvalue (`|CreateWidget` "/Game/Blueprints/Crosshair.Crosshair_C"))
  (`UserWidget.AddToViewport` _returnvalue 0)
  (bind _returnvalue_2 (`self.getMoveMaxSpeed`))
  (bind _output_get (set `self.DefaultSpeed` _returnvalue_2))
  (`KismetSystemLibrary.PrintString` (`KismetStringLibrary.Conv_DoubleToString` _output_get)))

(event `EnhancedInput|/Game/Input/Actions/IA_Shoot`
  (params (ActionValue :type Boolean) (ElapsedSeconds :type "Float (double-precision)") (TriggeredSeconds :type "Float (double-precision)") (InputAction :type "InputAction Object Reference" :default "/Game/Input/Actions/IA_Shoot.IA_Shoot")))

(event `/Game/Blueprints/Enviornmental_Hazards/BP_HazardTrigger.EnteredHazardZone`
  (params (HazardActorIn :type "Actor Object Reference") (ForceStrengthIn :type "Float (double-precision)") (ForceVector :type "Vector Structure"))
  (bind _movementcomponent (`self.MovementComponent`))
  (bind _movementcomponent_2 (`self.MovementComponent`))
  (`/Engine/EditorBlueprintResources/StandardMacros.FlipFlop`
    (:`A`
      (set `self.Force Vector` ForceVector)
      (bind _output_get (set `self.Force Strength In` ForceStrengthIn))
      (`KismetSystemLibrary.PrintString` (`KismetStringLibrary.Concat_StrStr` "Enterered triggerbox " "Object: " (`KismetSystemLibrary.GetDisplayName` HazardActorIn) "Force Strength: " (`KismetStringLibrary.Conv_DoubleToString` _output_get)))
      (set `self.bIsInGeyser` true)
      (set `FloatingPawnMovement.MaxSpeed` 5000.0 _movementcomponent)
      (set `FloatingPawnMovement.Acceleration` (* (`self.DefaultSpeed`) (`self.Force Strength In`)) _movementcomponent))
    (:`B`
      (`KismetSystemLibrary.PrintString` "Left TriggerBox")
      (set `self.bIsInGeyser` false)
      (bind _output_get_2 (set `FloatingPawnMovement.MaxSpeed` (`self.DefaultSpeed`) (`self.MovementComponent`)))
      (`KismetSystemLibrary.PrintString` (`KismetStringLibrary.Conv_DoubleToString` _output_get_2))
      (set `FloatingPawnMovement.MaxSpeed` (`self.DefaultSpeed`) _movementcomponent_2)
      (set `FloatingPawnMovement.Acceleration` 500.0 _movementcomponent_2))))

(event `self.ReceiveTick`
  (params (DeltaSeconds :type "Float (single-precision)"))
  (if (`self.bIsInGeyser`)
    (`self.GeyserForce`)))

(event `EnhancedInput|/Game/Input/Actions/IA_Interact`
  (params (ActionValue :type Boolean) (ElapsedSeconds :type "Float (double-precision)") (TriggeredSeconds :type "Float (double-precision)") (InputAction :type "InputAction Object Reference" :default "/Game/Input/Actions/IA_Interact.IA_Interact")))

(event `HighlightTimerSwitch`
  (`/Engine/EditorBlueprintResources/StandardMacros.FlipFlop`
    (:`A`
      (`KismetSystemLibrary.PrintString` "on")
      (`KismetSystemLibrary.K2_SetTimerDelegate` (delegate `TimerRunning`) 0.1 true))
    (:`B`
      (`KismetSystemLibrary.PrintString` "off"))))

(event `TimerRunning`
  (`self.TimerInteractHighlight`))

(fn `GeyserForce`
  (`PawnMovementComponent.AddInputVector` (`self.MovementComponent`) (`self.Force Vector`) false))

(fn `OnInteractHighlight`
  (params (bCanInteract :type Boolean :default false))
  (return))

(fn `TimerInteractHighlight`
  (bind _interactableactors (`self.InteractableActors`))
  (for (_array_element _array_index) _interactableactors
    (if (== _array_index 0)
      (bind _returnvalue (`KismetMathLibrary.Vector_Distance` (`SceneComponent.K2_GetComponentLocation` (`self.GetComponentByClass` _array_element "/Script/Engine.StaticMeshComponent")) (`SceneComponent.K2_GetComponentLocation` (`self.Arrow`))))
      (set `self.ClosestValue` _returnvalue)
      (set `self.CurrentHighlightActor` 0)
      (else
        (bind _output_get (set `self.CompareValue` _returnvalue))
        (if (< _output_get (`self.ClosestValue`))
          (set `self.ClosestValue` (`self.CompareValue`))
          (set `self.CurrentHighlightActor` _array_index)))))
  (for (_array_element_2 _array_index_2) _interactableactors
    (if (== _array_index_2 (`self.CurrentHighlightActor`))
      (message `/Game/Blueprints/BPI_HighlightInteraction.OnInteractHighlight` _array_element_2 true)
      (else
        (message `/Game/Blueprints/BPI_HighlightInteraction.OnInteractHighlight` _array_element_2 false)))))

(fn `UserConstructionScript`)