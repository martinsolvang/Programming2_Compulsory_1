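; BP_Projectile is a water bubble projectile that grows in flight and pops into small bubbles on impact.
; Tick enlarges the WaterBubble component at a steady rate until its scale passes a cap and latches the TooBig flag.
; A Sphere hit hides the bubble, stops the FollowBubbles effect and briefly activates SmallBubbles, then sets a short lifespan to clean up the actor.
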(event `self.ReceiveTick`
  (params (DeltaSeconds :type "Float (single-precision)"))
  (bind _waterbubble (`self.WaterBubble`))
  (bind _returnvalue (`SceneComponent.K2_GetComponentScale` _waterbubble))
  (if (not (`self.bTooBig`))
    (`SceneComponent.SetWorldScale3D` _waterbubble (+ _returnvalue (* DeltaSeconds 2.0)))
    (if (> (.x _returnvalue) 2.0)
      (set `self.bTooBig` true))))

(event `self.Sphere.OnComponentHit`
  (params (HitComponent :type "PrimitiveComponent Object Reference") (OtherActor :type "Actor Object Reference") (OtherComp :type "PrimitiveComponent Object Reference") (NormalImpulse :type "Vector Structure") (Hit :type "HitResult Structure (by ref)"))
  (`ActorComponent.Activate` (`self.Small bubbles`) false)
  (`SceneComponent.SetVisibility` (`self.WaterBubble`) false false)
  (`ActorComponent.Deactivate` (`self.FollowBubbles`))
  (`KismetSystemLibrary.Delay` 0.2)
  (`ActorComponent.Deactivate` (`self.Small bubbles`))
  (`self.SetLifeSpan` 5.0))

(fn `UserConstructionScript`)