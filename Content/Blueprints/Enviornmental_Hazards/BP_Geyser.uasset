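; BP_Geyser is an environmental hazard actor that passes a directional force to actors overlapping it.
; On begin overlap, it sends EnteredHazardZoneMessage through the BP_HazardTrigger interface with itself, ForceStrength and the forward vector of ForceDirection.
; End overlap reuses the same message with a zero vector to signal no force, as the receiving actor handles the force itself.
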(event `self.ReceiveActorBeginOverlap`
  (params (OtherActor :type "Actor Object Reference"))
  (if (`KismetSystemLibrary.DoesImplementInterface` OtherActor "/Game/Blueprints/Enviornmental_Hazards/BP_HazardTrigger.BP_HazardTrigger_C")
    (message `/Game/Blueprints/Enviornmental_Hazards/BP_HazardTrigger.EnteredHazardZone` OtherActor self (`self.Force Strength`) (`SceneComponent.GetForwardVector` (`self.ForceDirection`)))))

(event `self.ReceiveActorEndOverlap`
  (params (OtherActor :type "Actor Object Reference"))
  (if (`KismetSystemLibrary.DoesImplementInterface` OtherActor "/Game/Blueprints/Enviornmental_Hazards/BP_HazardTrigger.BP_HazardTrigger_C")
    (message `/Game/Blueprints/Enviornmental_Hazards/BP_HazardTrigger.EnteredHazardZone` OtherActor self (`self.Force Strength`) (0.0 0.0 0.0))))

(fn `UserConstructionScript`)